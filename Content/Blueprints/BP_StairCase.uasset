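; Procedural staircase actor that builds a row of step meshes in its construction script, with no active runtime logic.
; A loop driven by NumSteps adds static mesh components, attaches them to Stair and spaces them along local X by mesh width plus spacing.
; Each step's local Y scale grows with its index, and a negative half-height Y offset per index compensates for the stretch.
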(event `self.ReceiveBeginPlay`)

(event `self.ReceiveActorBeginOverlap`
  (params (OtherActor :type "Actor Object Reference")))

(event `self.ReceiveTick`
  (params (DeltaSeconds :type "Float (single-precision)")))

(fn `UserConstructionScript`
  (for _index (range (+ (`self.NumSteps`) 1))
    (bind _returnvalue (`AddComponent|Static Mesh Component_694`))
    (bind _output_get (set `self.GeneratedStair` _returnvalue))
    (`SceneComponent.SetRelativeScale3D` _output_get (`KismetMathLibrary.MakeVector` 1.0 (`KismetMathLibrary.Conv_IntToDouble` (+ _index 1)) 1.0))
    (`SceneComponent.K2_AttachTo` (`self.GeneratedStair`) (`self.Stair`) "None" "KeepRelativeOffset" true)
    (`SceneComponent.K2_SetRelativeLocation` (`self.GeneratedStair`) (`KismetMathLibrary.MakeVector` (* _index (+ (`self.StepMeshWidth`) (`self.StepSpacing`))) (* _index (* (`self.StepMeshHeight`) -0.5))) false)))