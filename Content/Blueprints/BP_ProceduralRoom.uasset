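; BP_ProceduralRoom is a configurable modular room actor with a floor, ceiling, four walls and four supports.
; The construction script assigns each piece's static mesh component its own mesh variable when that piece's toggle is on, and clears the mesh when off.
; A sequence handles the floor, ceiling and walls first, then the supports.
; The event graph holds only disabled stub events, so nothing runs during play.
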(event `self.ReceiveBeginPlay`)

(event `self.ReceiveActorBeginOverlap`
  (params (OtherActor :type "Actor Object Reference")))

(event `self.ReceiveTick`
  (params (DeltaSeconds :type "Float (single-precision)")))

(fn `UserConstructionScript`
  (bind _ceilling (`self.Ceilling`))
  (bind _wall1 (`self.Wall1`))
  (bind _wall2 (`self.Wall2`))
  (bind _wall3 (`self.Wall3`))
  (bind _wall4 (`self.Wall4`))
  (bind _support1 (`self.Support1`))
  (bind _support2 (`self.Support2`))
  (bind _support3 (`self.Support3`))
  (bind _support4 (`self.Support4`))
  (bind _floor (`self.Floor`))
  (`|ExecutionSequence`
    (:`then_0`
      ;[1 1 1] Setting the walls
      (if (`self.Floor?`)
        (`StaticMeshComponent.SetStaticMesh` _floor (`self.FloorMesh`))
        (else
          (`StaticMeshComponent.SetStaticMesh` _floor null)))
      (if (`self.Celiing?`)
        (`StaticMeshComponent.SetStaticMesh` _ceilling (`self.CeillingMesh`))
        (else
          (`StaticMeshComponent.SetStaticMesh` _ceilling null)))
      (if (`self.Wall1?`)
        (`StaticMeshComponent.SetStaticMesh` _wall1 (`self.WallMesh1`))
        (else
          (`StaticMeshComponent.SetStaticMesh` _wall1 null)))
      (if (`self.Wall2?`)
        (`StaticMeshComponent.SetStaticMesh` _wall2 (`self.WallMesh2`))
        (else
          (`StaticMeshComponent.SetStaticMesh` _wall2 null)))
      (if (`self.Wall3?`)
        (`StaticMeshComponent.SetStaticMesh` _wall3 (`self.WallMesh3`))
        (else
          (`StaticMeshComponent.SetStaticMesh` _wall3 null)))
      (if (`self.Wall4?`)
        (`StaticMeshComponent.SetStaticMesh` _wall4 (`self.WallMesh4`))
        (else
          (`StaticMeshComponent.SetStaticMesh` _wall4 null))))
    (:`then_1`
      (if (`self.Support1?`)
        (`StaticMeshComponent.SetStaticMesh` _support1 (`self.Support1Mesh`))
        (else
          (`StaticMeshComponent.SetStaticMesh` _support1 null)))
      (if (`self.Support2?`)
        (`StaticMeshComponent.SetStaticMesh` _support2 (`self.Support2Mesh`))
        (else
          (`StaticMeshComponent.SetStaticMesh` _support2 null)))
      (if (`self.Support3?`)
        (`StaticMeshComponent.SetStaticMesh` _support3 (`self.Support3Mesh`))
        (else
          (`StaticMeshComponent.SetStaticMesh` _support3 null)))
      (if (`self.Support4?`)
        (`StaticMeshComponent.SetStaticMesh` _support4 (`self.Support4Mesh`))
        (else
          (`StaticMeshComponent.SetStaticMesh` _support4 null))))))