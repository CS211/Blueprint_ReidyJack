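; BP_ProceduralRoom is a modular room actor that assembles itself in the Construction Script from toggles for floor, ceiling, four walls and four supports.
; It assigns meshes, then IsMeshPresent sets each piece's visibility and collision together.
; Support mesh size follows the presence of floor and ceiling, with supports offset downward when the floor is absent.
; Shown walls gain top or bottom filler pieces where the ceiling or floor is missing.
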(event `self.ReceiveBeginPlay`)

(event `self.ReceiveActorBeginOverlap`
  (params (OtherActor :type "Actor Object Reference")))

(event `self.ReceiveTick`
  (params (DeltaSeconds :type "Float (single-precision)")))

(fn `InitializeSupports`
  (`StaticMeshComponent.SetStaticMesh` (`self.Support1`) (`self.SupportStaticMesh`))
  (`self.IsMeshPresent` (`self.Support1?`) (`self.Support1`))
  (`StaticMeshComponent.SetStaticMesh` (`self.Support2`) (`self.SupportStaticMesh`))
  (`self.IsMeshPresent` (`self.Support2?`) (`self.Support2`))
  (`StaticMeshComponent.SetStaticMesh` (`self.Support3`) (`self.SupportStaticMesh`))
  (`self.IsMeshPresent` (`self.Support3?`) (`self.Support3`))
  (`StaticMeshComponent.SetStaticMesh` (`self.Support4`) (`self.SupportStaticMesh`))
  (`self.IsMeshPresent` (`self.Support4?`) (`self.Support4`)))

(fn `InitializeWallMeshes`
  (`StaticMeshComponent.SetStaticMesh` (`self.Floor`) (`self.FloorMesh`))
  (`StaticMeshComponent.SetStaticMesh` (`self.Ceilling`) (`self.CeillingMesh`))
  (`StaticMeshComponent.SetStaticMesh` (`self.Wall1`) (`self.WallMesh1`))
  (`StaticMeshComponent.SetStaticMesh` (`self.Wall2`) (`self.WallMesh2`))
  (`StaticMeshComponent.SetStaticMesh` (`self.Wall3`) (`self.WallMesh3`))
  (`StaticMeshComponent.SetStaticMesh` (`self.Wall4`) (`self.WallMesh4`)))

(fn `IsMeshPresent`
  (params (IsShown :type Boolean :default false) (StaticMeshComponent :type "StaticMeshComponent Object Reference"))
  (`SceneComponent.SetVisibility` StaticMeshComponent IsShown false)
  (if IsShown
    (`PrimitiveComponent.SetCollisionEnabled` StaticMeshComponent "QueryAndPhysics")
    (else
      (`PrimitiveComponent.SetCollisionEnabled` StaticMeshComponent "NoCollision"))))

(fn `ResizeSupports`
  (if (`self.Floor?`)
    (if (`self.Celiing?`)
      (set `self.SupportStaticMesh` (`self.SmallSupportMesh`))
      (else
        (set `self.SupportStaticMesh` (`self.MediumSupportMesh`))))
    (else
      (if (`self.Celiing?`)
        (set `self.SupportStaticMesh` (`self.MediumSupportMesh`))
        (else
          (set `self.SupportStaticMesh` (`self.LargeSupportMesh`))))
      (`SceneComponent.K2_AddLocalOffset` (`self.Support1`) (0.0 0.0 -25.0) false)
      (`SceneComponent.K2_AddLocalOffset` (`self.Support2`) (0.0 0.0 -25.0) false)
      (`SceneComponent.K2_AddLocalOffset` (`self.Support3`) (0.0 0.0 -25.0) false)
      (`SceneComponent.K2_AddLocalOffset` (`self.Support4`) (0.0 0.0 -25.0) false))))

(fn `ResizeWalls`
  (`|ExecutionSequence`
    (:`then_0`
      (`self.IsMeshPresent` (and (`self.Wall1?`) (not (`self.Celiing?`))) (`self.Wall1FillTop`))
      (`self.IsMeshPresent` (and (`self.Wall1?`) (not (`self.Floor?`))) (`self.Wall1FillBottom`)))
    (:`then_1`
      (`self.IsMeshPresent` (and (`self.Wall2?`) (not (`self.Celiing?`))) (`self.Wall2FillTop`))
      (`self.IsMeshPresent` (and (`self.Wall2?`) (not (`self.Floor?`))) (`self.Wall2FillBottom`)))
    (:`then_2`
      (`self.IsMeshPresent` (and (`self.Wall3?`) (not (`self.Celiing?`))) (`self.Wall3FillTop`))
      (`self.IsMeshPresent` (and (`self.Wall3?`) (not (`self.Floor?`))) (`self.Wall3FillBottom`)))
    (:`then_3`
      (`self.IsMeshPresent` (and (`self.Wall4?`) (not (`self.Celiing?`))) (`self.Wall4FillTop`))
      (`self.IsMeshPresent` (and (`self.Wall4?`) (not (`self.Floor?`))) (`self.Wall4FillBottom`)))))

(fn `SetWallVisibilities`
  (`self.IsMeshPresent` (`self.Floor?`) (`self.Floor`))
  (`self.IsMeshPresent` (`self.Celiing?`) (`self.Ceilling`))
  (`self.IsMeshPresent` (`self.Wall1?`) (`self.Wall1`))
  (`self.IsMeshPresent` (`self.Wall2?`) (`self.Wall2`))
  (`self.IsMeshPresent` (`self.Wall3?`) (`self.Wall3`))
  (`self.IsMeshPresent` (`self.Wall4?`) (`self.Wall4`)))

(fn `UserConstructionScript`
  ;[1 1 1] Setting the walls
  (`|ExecutionSequence`
    (:`then_0`
      (`self.InitializeWallMeshes`))
    (:`then_1`
      (`self.SetWallVisibilities`))
    (:`then_2`
      (`self.ResizeSupports`))
    (:`then_3`
      (`self.InitializeSupports`))
    (:`then_4`
      (`self.ResizeWalls`))))