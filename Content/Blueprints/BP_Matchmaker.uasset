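; BP_Matchmaker is a trigger that puts the first local player into a two-connection LAN session when anything begins overlapping its Box component.
; The overlap runs an async session search, then joins the first result if any exist.
; With no results, it creates a session and opens the level named by LevelString as a listen server.
; Search and creation failures only print debug strings.
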(event `self.Box.OnComponentBeginOverlap`
  (params (OtherActor :type "Actor Object Reference") (OtherComp :type "PrimitiveComponent Object Reference") (OtherBodyIndex :type Integer) (bFromSweep :type Boolean) (SweepResult :type "EngineTypes.HitResult Structure (by ref)"))
  (`KismetSystemLibrary.PrintString` "Hello")
  (bind _results (`FindSessionsCallbackProxy.FindSessions` (`GameplayStatics.GetPlayerController` 0) 20 true)
    (:`OnSuccess`
      (if (== (`KismetArrayLibrary.Array_Length` _results) 0)
        (`CreateSessionCallbackProxy.CreateSession` (`GameplayStatics.GetPlayerController` 0) 2 true
          (:`OnSuccess`
            (`GameplayStatics.OpenLevel` (`self.LevelString`) true "listen"))
          (:`OnFailure`
            (`KismetSystemLibrary.PrintString` "Create Session Fail")))
        (else
          (`JoinSessionCallbackProxy.JoinSession` (`GameplayStatics.GetPlayerController` 0) (`KismetArrayLibrary.Array_Get` _results)))))
    (:`OnFailure`
      (`KismetSystemLibrary.PrintString` "SessionFails"))))

(fn `UserConstructionScript`)